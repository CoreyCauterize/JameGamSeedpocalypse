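; BP_NPC_Applicant is an applicant NPC that feeds its resume data to the questions UI and can turn into a swan.
; Shortly after BeginPlay, it passes its applicant data to the first BP_Questions widget found.
; SwanSwap changes its mesh to the Swan asset, then spawns a collision-free Character with the same mesh, attached at the "Swan" socket and rotated.
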(event EventBeginPlay
  (Utilities|FlowControl|Delay 0.5)
  (bind _returnvalue (Class|NPCApplicant|GetApplicantData))
  (bind _foundwidgets (Widget|GetAllWidgetsOfClass "/Game/Blueprints/HUD/BP_Questions.BP_Questions_C" false))
  (Default|UpdateResume (Utilities|Array|Get(acopy) _foundwidgets) _returnvalue))

(event Collision|EventActorBeginOverlap
  (params (OtherActor :type Actor%20Object%20Reference)))

(event EventTick
  (params (DeltaSeconds :type Float%20%28single-precision%29)))

(fn ConstructionScript)

(fn SwanSwap
  (Variables|/Script/Engine.SkeletalMeshComponent|SetSkeletalMeshAsset (Variables|Character|GetMesh) "/Game/NPC/Swan.Swan")
  (bind _returnvalue (Game|SpawnActorfromClass "/Script/Engine.Character" (Transformation|GetActorTransform) "AlwaysSpawn" "MultiplyWithRoot" 0 0))
  (Collision|SetActorEnableCollision _returnvalue false)
  (Variables|/Script/Engine.SkeletalMeshComponent|SetSkeletalMeshAsset (Variables|/Script/Engine.Character|GetMesh _returnvalue) "/Game/NPC/Swan.Swan")
  (Transformation|AttachActorToActor _returnvalue self "Swan" "SnapToTarget" "SnapToTarget" "KeepRelative" true)
  (Transformation|SetRelativeRotation (Variables|/Script/Engine.Character|GetMesh _returnvalue) "0.000000,-90.000000,0.000000" false false))